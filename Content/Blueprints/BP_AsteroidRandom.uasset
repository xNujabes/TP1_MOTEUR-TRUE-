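; BP_AsteroidRandom is a shootable asteroid that awards score to the player ship when its health runs out.
; Overlaps with BP_Projectile apply damage, play a hit sound with sparks and destroy the projectile.
; At zero health it plays explosion effects and sounds and adds ScoreValue to the BP_PlayerShip found by class lookup.
; This graph contains no randomization and never destroys the asteroid itself.
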(event `self.ReceiveActorBeginOverlap`
  (params (OtherActor :type "Actor Object Reference"))
  (bind _returnvalue (`self.K2_GetActorLocation`))
  (bind _asbp_projectile (cast `/Game/Blueprints/BP_Projectile` OtherActor))
  (`self.TakeDamage` 1.0)
  (`GameplayStatics.PlaySoundAtLocation` "/Engine/EngineSounds/1kSineTonePing.1kSineTonePing" _returnvalue (struct) 1.0 1.0 0.0 null null null null)
  (`GameplayStatics.SpawnEmitterAtLocation` "/Game/StarterContent/Particles/P_Sparks.P_Sparks" (`self.K2_GetActorLocation` _asbp_projectile))
  (`self.K2_DestroyActor` _asbp_projectile)
  (if (== 0 (`self.Health`))
    (`GameplayStatics.PlaySoundAtLocation` "/Game/StarterContent/Audio/Explosion02.Explosion02" _returnvalue (struct) 1.0 1.0 0.0 null null null null)
    (`GameplayStatics.SpawnEmitterAtLocation` "/Game/StarterContent/Particles/P_Explosion.P_Explosion" _returnvalue (struct) (1.5 1.5 1.5))
    (bind _returnvalue_2 (`GameplayStatics.GetActorOfClass` "/Game/Blueprints/BP_PlayerShip.BP_PlayerShip_C"))
    (`PlayerShip.AddScore` _returnvalue_2 (`self.ScoreValue`))
    (`GameplayStatics.PlaySound2D` "/Engine/VREditor/Sounds/UI/Camera_Shutter.Camera_Shutter" 1.0 1.0 0.0 null null)))

(fn `UserConstructionScript`)