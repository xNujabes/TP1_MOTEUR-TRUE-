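; BP_PlayerShip is the player's ship, which loses health when asteroids collide with it.
; On overlap with an Asteroid, it plays a sound and spark effect, destroys the asteroid and takes one point of damage.
; When Health equals zero, it shows the GameOver widget, switches input to UI only and pauses the game.
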(event `self.ReceiveActorBeginOverlap`
  (params (OtherActor :type "Actor Object Reference"))
  (bind _returnvalue (`self.K2_GetActorLocation`))
  (bind _asasteroid (cast `Asteroid` OtherActor))
  (`GameplayStatics.PlaySoundAtLocation` "/Engine/VREditor/Sounds/VR_negative.VR_negative" _returnvalue (struct) 1.0 1.0 0.0 null null null null)
  (`GameplayStatics.SpawnEmitterAtLocation` "/Game/StarterContent/Particles/P_Sparks.P_Sparks" _returnvalue (struct) (3.0 3.0 3.0))
  (`self.K2_DestroyActor` _asasteroid)
  (`self.TakeDamage` 1.0)
  (if (== (`self.Health`) 0)
    (bind _returnvalue_2 (`|CreateWidget` "/Game/UI/GameOver.GameOver_C"))
    (bind _output_get (set `self.NewVar` _returnvalue_2))
    (`UserWidget.AddToViewport` _output_get 0)
    (`WidgetBlueprintLibrary.SetInputMode_UIOnlyEx` (`GameplayStatics.GetPlayerController` 0) null)
    (`GameplayStatics.SetGamePaused` true)))

(fn `UserConstructionScript`)